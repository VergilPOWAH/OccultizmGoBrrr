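; BP_ky_fireBall is a fireball projectile that flies forward and explodes on overlapping any valid actor other than its instigator.
; BeginPlay spawns a colored shockwave and plays a timeline whose curve scales the per-Tick forward movement.
; Tick also counts down LifeTime, which a Delay loop polls to disable collision, deactivate the effect and destroy the actor.
; An overlap spawns the hit effect, calls Explode with Damage, then destroys it; construction assigns Sphere as DamageArea.
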(event `self.ReceiveBeginPlay`
  (bind _defaultsceneroot (`self.DefaultSceneRoot`))
  ;[1 1 1] spawn shot shockwave
  (bind _returnvalue (`GameplayStatics.SpawnEmitterAtLocation` "/Game/FXVarietyPack/Particles/P_ky_shotShockwave.P_ky_shotShockwave" (`SceneComponent.K2_GetComponentLocation` _defaultsceneroot) (`SceneComponent.K2_GetComponentRotation` _defaultsceneroot)))
  (`ParticleSystemComponent.SetVectorParameter` _returnvalue "color" (`KismetMathLibrary.Conv_LinearColorToVector` (`self.color`)))
  ;[1 1 1] effect move correct
  (bind (_direction _valuecorrect) (`Timeline|Timeline_0`)
    (:`Update`
      (set `self.speedCorrect` _valuecorrect)
      ;[1 1 1] duration control
      (`KismetSystemLibrary.Delay` 0.1 :!label _label)
      (if (< (`self.LifeTime`) 0.0)
        ;[1 1 1] fx deactivate
        (`PrimitiveComponent.SetCollisionEnabled` (`self.Box`) "NoCollision")
        (`ActorComponent.Deactivate` (`self.FX1`))
        (`KismetSystemLibrary.Delay` 1.0)
        ;[1 1 1] effect destroy
        (`self.K2_DestroyActor`)
        (else
          (goto _label))))))

(event `self.ReceiveTick`
  (params (DeltaSeconds :type "Float (single-precision)"))
  ;[1 1 1] duration increment for control
  (set `self.LifeTime` (- (`self.LifeTime`) DeltaSeconds))
  ;[1 1 1] move control
  (`self.K2_AddActorLocalOffset` (`KismetMathLibrary.MakeVector` (* (`self.Speed`) (`self.speedCorrect`) (`GameplayStatics.GetWorldDeltaSeconds`)))))

(event `self.ReceiveActorBeginOverlap`
  (params (OtherActor :type "Actor Object Reference"))
  ;[1 1 1] spawn collison fx
  (if (`KismetSystemLibrary.IsValid` OtherActor)
    (if (!= OtherActor (`self.GetInstigator`))
      (`GameplayStatics.SpawnEmitterAtLocation` (`self.hitFx`) (`SceneComponent.K2_GetComponentLocation` (`self.Box`)))
      (`self.Explode` (`self.Instigator`) (`self.Damage`))
      ;[1 1 1] fx destroy
      (`self.K2_DestroyActor`))))

(fn `UserConstructionScript`
  (set `self.DamageArea` (`self.Sphere`)))